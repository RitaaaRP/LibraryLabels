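; Actor component that detects which BP_InterantionArea the player camera is looking at and toggles its focus.
; Each tick it line-traces forward from the camera manager by Length on the Visibility channel, with debug drawing enabled.
; Hit actors passing its checks become FocusedActor, and a class test decides whether to focus or clear.
; TraceInteractionArea unfocuses the previous area, focuses the new one, and clears cached references when focus is lost.
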(event EventTick
  (params (DeltaSeconds :type Float%20%28single-precision%29))
  (CallFunction|Trace))

(fn Trace
  (bind _returnvalue (Game|GetPlayerCameraManager 0))
  (bind _returnvalue_2 (Transformation|GetActorLocation _returnvalue))
  (bind (_outhit _returnvalue_3) (Collision|LineTraceByChannel _returnvalue_2 (+ _returnvalue_2 (* (Math|Vector|GetForwardVector (Transformation|GetActorRotation _returnvalue)) (Variables|Default|GetLength))) "TraceTypeQuery1" false 0 "ForDuration"))
  (if _returnvalue_3
    (if (!= (Variables|Default|GetFocusedActor) 0)
      (Variables|Default|SetFocusedActor (.HitActor (Collision|BreakHitResult _outhit)))
      (CallFunction|TraceInteractionArea (== (Utilities|GetClass (.HitActor (Collision|BreakHitResult _outhit))) 0)))
    (else
      (CallFunction|TraceInteractionArea false))))

(fn TraceInteractionArea
  (params (Trace :type Boolean))
  (if Trace
    (if (Variables|Default|GetIsTracinngInteractionArea)
      (Default|ToggleFocuse (Variables|Default|GetFocusedInteractionArea) false))
    (bind _asbp_interantion_area (Utilities|Casting|CastToBP_InterantionArea (Variables|Default|GetFocusedActor)))
    (bind _output_get (Variables|Default|SetFocusedInteractionArea _asbp_interantion_area))
    (Default|ToggleFocuse _output_get true)
    (Variables|Default|SetIsTracinngInteractionArea true)
    (elif (Variables|Default|GetIsTracinngInteractionArea)
      (Variables|Default|SetIsTracinngInteractionArea false)
      (Default|ToggleFocuse (Variables|Default|GetFocusedInteractionArea) false)
      (Variables|Default|SetFocusedActor 0)
      (Variables|Default|SetFocusedInteractionArea 0))))